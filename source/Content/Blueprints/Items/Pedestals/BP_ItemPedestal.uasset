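; Interactable item pedestal that displays an item from the player's inventory in the world.
; Interacting stores the player and opens their inventory display, which closes when they end overlap.
; PlaceItem checks inventory, spawns the Blueprint from DT_ItemResource at ItemPlacement and removes one, while TakeItem returns it and destroys the actor.
; PlaceNewItem spawns an item's WorldItemRef directly, without touching inventory.
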(event Custom|Event%20PlaceNewItem
  (params (NewItem :type STRUCT%20Base%20Items%20Structure))
  (bind _returnvalue (Game|SpawnActorfromClass (.worlditemref NewItem) (Transformation|GetWorldTransform (Variables|Default|GetItemPlacement)) "Undefined" "MultiplyWithRoot" 0 "NewEnumerator0" 0))
  (Variables|Default|SetCurrentlyPlacedItem _returnvalue))

(event Custom|PlaceItem
  (params (Item :type E_Items%20Enum :default "NewEnumerator0"))
  (bind (_itemcount _inventoryindex _haveitem_) (Default|FindItem(user) (Variables|/Game/Blueprints/Characters/HeroCharacter/BP_PlayerCharacter.BP_PlayerCharacter_C|GetBP_InventoryV2 (Variables|Default|GetPlayerReference)) Item))
  (if _haveitem_
    (if (> _itemcount 0)
      (bind _returnvalue (Utilities|GetDataTableRow "/Game/Blueprints/Systems/Inventory/DT_ItemResource.DT_ItemResource" (Utilities|String|StringToName (Utilities|String|ToString(Integer) (Math|Conversions|ToInteger(Byte) Item))))
        (:then
          (bind _returnvalue_2 (Game|SpawnActorfromClass (.blueprint _returnvalue) (Transformation|GetWorldTransform (Variables|Default|GetItemPlacement)) "Undefined" "MultiplyWithRoot" 0 Item 0))
          (Variables|Default|SetCurrentlyPlacedItem _returnvalue_2)
          (Default|RemovefromInventory(user) (Variables|/Game/Blueprints/Characters/HeroCharacter/BP_PlayerCharacter.BP_PlayerCharacter_C|GetBP_InventoryV2 (Variables|Default|GetPlayerReference)) Item 1))))))

(event Custom|TakeItem
  (Default|AddtoInventory(user) (Variables|/Game/Blueprints/Characters/HeroCharacter/BP_PlayerCharacter.BP_PlayerCharacter_C|GetBP_InventoryV2 (Variables|Default|GetPlayerReference)) (Variables|/Game/Blueprints/Items/Pickups/BP_BasePickupItem.BP_BasePickupItem_C|GetItem_ID (Variables|Default|GetCurrentlyPlacedItem)))
  (Actor|DestroyActor (Variables|Default|GetCurrentlyPlacedItem))
  (Variables|Default|SetCurrentlyPlacedItem 0))

(event EventBeginPlay)

(event Collision|EventActorBeginOverlap
  (params (OtherActor :type Actor%20Object%20Reference)))

(event EventOnInteract
  (params (Interactor :type Object%20Object%20Reference))
  (bind _asbp_player_character (Utilities|Casting|CastToBP_PlayerCharacter Interactor))
  (Variables|Default|SetPlayerReference _asbp_player_character)
  (Default|HandleInventoryDisplay _asbp_player_character true))

(event Collision|EventActorEndOverlap
  (params (OtherActor :type Actor%20Object%20Reference))
  (|CallParentFunction OtherActor)
  (bind _asbp_player_character (Utilities|Casting|CastToBP_PlayerCharacter OtherActor))
  (Default|HandleInventoryDisplay _asbp_player_character false))

(fn ConstructionScript)

(fn GetDisplayText
  (return "Display Item"))