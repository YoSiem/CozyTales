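; Base pickup item actor that the player interacts with to add it to their inventory.
; On interaction by a player character, it plays a pickup sound, schedules its own destruction after a short delay, and passes its ItemID to the inventory component.
; An interaction zone acts as a tether: when the physics mesh leaves it, its velocities are zeroed and it snaps back to the zone's location.
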(event OnComponentEndOverlap(InteractionZone)
  (params (OverlappedComponent :type Primitive%20Component%20Object%20Reference) (OtherActor :type Actor%20Object%20Reference) (OtherComp :type Primitive%20Component%20Object%20Reference) (OtherBodyIndex :type Integer))
  (if (== OtherComp (Variables|Default|GetMesh))
    (CallFunction|ResetItemMeshPosition)))

(event Custom|Destroy%20Item
  (Utilities|FlowControl|Delay 0.1)
  (Actor|DestroyActor))

(event EventOnInteract
  (params (Interactor :type Object%20Object%20Reference))
  (bind _asbp_player_character (Utilities|Casting|CastToBP_PlayerCharacter Interactor))
  (bind _item_id (CallFunction|PickUpItem))
  (Default|AddtoInventory(user) (Variables|/Game/Blueprints/Characters/HeroCharacter/BP_PlayerCharacter.BP_PlayerCharacter_C|GetBP_InventoryV2 _asbp_player_character) _item_id))

(fn ConstructionScript)

(fn ResetItemMeshPosition
  (bind _mesh (Variables|Default|GetMesh))
  (Physics|SetPhysicsLinearVelocity _mesh "0, 0, 0" false "None")
  (Class|PrimitiveComponent|SetPhysicsAngularVelocityinRadians _mesh "0, 0, 0" false "None")
  (Transformation|SetWorldLocation _mesh (Transformation|GetWorldLocation (Variables|Default|GetInteractionZone)) false false))

(fn GetDisplayText
  (return "Pick up"))

(fn PickUpItem
  (Audio|SpawnSoundatLocation "/Game/Sounds/MetaSounds/MSP_Pick_Item.MSP_Pick_Item" (Transformation|GetActorLocation) "0, 0, 0" 1.0 1.0 0.0 0 0)
  (Development|PrintString "Item picked")
  (CallFunction|DestroyItem)
  (return (Variables|Default|GetItem_ID)))