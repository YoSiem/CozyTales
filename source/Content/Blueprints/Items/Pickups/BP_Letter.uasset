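; BP_Letter is an interactable pickup the player reads, opening a WBP_Letter widget and enabling mouse input.
; On interact it creates the widget once, then for non-starter letters adds pages from every key of the letter text's string table, or the raw text if it has none.
; A second branch of the interaction updates the status of each quest in its QuestsToModify map through the quest manager.
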(event EventBeginPlay)

(event Collision|EventActorBeginOverlap
  (params (OtherActor :type Actor%20Object%20Reference))
  (|CallParentFunction OtherActor) ; This node is disabled and will not be called.\nDrag off pins to build functionality.
)

(event EventTick
  (params (DeltaSeconds :type Float%20%28single-precision%29)))

(event EventOnInteract
  (params (Interactor :type Object%20Object%20Reference))
  (bind _lettertext (Variables|Default|GetLetterText))
  (bind _quests_to_modify (Variables|QuestRelated|GetQuests%20To%20Modify))
  (bind (_outtableid _outkey _returnvalue) (Class|KismetTextLibrary|StringTableIdandKeyfromText _lettertext))
  (Utilities|FlowControl|Sequence
    (:then_0
      (bind _asbp_player_character (Utilities|Casting|CastToBP_PlayerCharacter Interactor))
      (Variables|Default|GetLetterWidgetRef
        (:then
          _)
        (:else
          (bind _returnvalue_2 (UserInterface|CreateWidget "/Game/UI/Widgets/WBP_Letter.WBP_Letter_C" (Variables|/Game/Blueprints/Characters/HeroCharacter/BP_PlayerCharacter.BP_PlayerCharacter_C|GetAs%20BP%20Controller _asbp_player_character)))
          (Variables|Default|SetLetterWidgetRef _returnvalue_2)))
      (if (Variables|Default|GetIsStarterLetter?)
        _
        (else
          (Default|EventonNotStarterLetter (Variables|Default|GetLetterWidgetRef))
          (if _returnvalue
            (for _array_element (Class|KismetStringTableLibrary|GetKeysfromStringTable _outtableid)
              (Default|EventAddPage (Variables|Default|GetLetterWidgetRef) (Class|KismetTextLibrary|TextfromStringTable _outtableid _array_element) (Variables|Default|GetShouldTextBeCentered?)))
            (else
              (Default|EventAddPage (Variables|Default|GetLetterWidgetRef) _lettertext (Variables|Default|GetShouldTextBeCentered?))))))
      (UserInterface|Viewport|AddtoViewport (Variables|Default|GetLetterWidgetRef) 0)
      (Default|EventShowLetter (Variables|Default|GetLetterWidgetRef))
      (bind _asbp_player_character_2 (Utilities|Casting|CastToBP_PlayerCharacter (Game|Player|GetPlayerPawn 0)))
      (Default|EnableMouseInput _asbp_player_character_2))
    (:then_1
      (bind _keys (Utilities|Map|Keys _quests_to_modify))
      (for _array_element_2 _keys
        (Default|UpdateQuestStatus (CallFunction|GetQuestManager) _array_element_2 (.Value (Utilities|Map|Find _quests_to_modify _array_element_2)))))))

(fn ConstructionScript
  (|CallParentFunction))

(fn PickUpItem
  (return "NewEnumerator0"))

(fn GetDisplayText
  (return "Read"))