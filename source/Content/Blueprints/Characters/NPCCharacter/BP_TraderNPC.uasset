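; Trader NPC that takes the player's fish on interaction and pays out item rewards once enough have been handed over.
; Each trade adds the fish to a running total, checked against the current DT_TradeTable1 row.
; Meeting the threshold advances the table index (wrapping to 1, not 0), plays the row's text as a monologue, grants the matching DT_ItemResource item and zeroes the total, discarding any surplus.
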(event Custom|Event%20DoTrade
  (params (Player :type BP%20Player%20Character%20Object%20Reference))
  (bind _bp_inventoryv2 (Variables|/Game/Blueprints/Characters/HeroCharacter/BP_PlayerCharacter.BP_PlayerCharacter_C|GetBP_InventoryV2 Player))
  (bind _itemcount (Default|FindItem(user) _bp_inventoryv2 "NewEnumerator3"))
  (Variables|Default|SetTradedFish (+ _itemcount (Variables|Default|GetTradedFish)))
  (CallFunction|HandleNewFishAmount)
  (Default|RemovefromInventory(user) _bp_inventoryv2 "NewEnumerator3" _itemcount))

(event Custom|Event%20TradeItem
  (params (ItemID :type Integer) (TradeText :type Text))
  (CallFunction|EventStartNpcMonologue (Utilities|Array|MakeArray (Utilities|Struct|MakeS_ConversationInfo TradeText)))
  (Utilities|FlowControl|Delay 0.2)
  (bind _outrownames (DataTable|GetDataTableRowNames "/Game/Blueprints/Systems/Inventory/DT_ItemResource.DT_ItemResource"))
  (bind _array_element (Utilities|Array|ForEachLoopwithBreak _outrownames :!label _label)
    (:LoopBody
      (bind _returnvalue (Utilities|GetDataTableRow "/Game/Blueprints/Systems/Inventory/DT_ItemResource.DT_ItemResource" _array_element)
        (:then
          (if (== (Math|Conversions|ToInteger(Byte) (.ID (Utilities|Struct|BreakS_ItemBase _returnvalue))) ItemID)
            (Variables|Default|SetReward%20ItemID (.ID (Utilities|Struct|BreakS_ItemBase _returnvalue)))
            (Variables|Default|SetFoundet? true)
            (goto _label Break)))))
    (:Completed
      (if (Variables|Default|GetFoundet?)
        (Default|AddtoInventory(user) (Variables|/Game/Blueprints/Characters/HeroCharacter/BP_PlayerCharacter.BP_PlayerCharacter_C|GetBP_InventoryV2 (Variables|Default|GetPlayerReferece)) (Variables|Default|GetReward%20ItemID))
        (CallFunction|ResetTradedFishCount)))))

(event EventBeginPlay
  (|CallParentFunction)
  (Rendering|SetVisibility (Variables|Default|GetActiveHighlight) true false)
  (CallFunction|SetConversationState true))

(event Collision|EventActorBeginOverlap
  (params (OtherActor :type Actor%20Object%20Reference))
  (|CallParentFunction OtherActor) ; This node is disabled and will not be called.\nDrag off pins to build functionality.
)

(event EventTick
  (params (DeltaSeconds :type Float%20%28single-precision%29)))

(event EventOnInteract
  (params (Interactor :type Object%20Object%20Reference))
  (bind _asbp_player_character (Utilities|Casting|CastToBP_PlayerCharacter Interactor))
  (bind _output_get (Variables|Default|SetPlayerReferece _asbp_player_character))
  (CallFunction|EventDoTrade _output_get))

(fn ConstructionScript
  (|CallParentFunction))

(fn HandleNewFishAmount
  (bind _outrownames (DataTable|GetDataTableRowNames "/Game/DataAssets/TradeTables/DT_TradeTable1.DT_TradeTable1"))
  (bind _returnvalue (Utilities|GetDataTableRow "/Game/DataAssets/TradeTables/DT_TradeTable1.DT_TradeTable1" (Utilities|Array|Get(acopy) _outrownames (Variables|Default|GetCurrentTradeItemIndex)))
    (:then
      (if (>= (Variables|Default|GetTradedFish) (.neededfishtotrade _returnvalue))
        (bind _outrownames_2 (DataTable|GetDataTableRowNames "/Game/Blueprints/Systems/Inventory/DT_ItemResource.DT_ItemResource"))
        (for _array_element _outrownames_2
          (bind _returnvalue_2 (Utilities|GetDataTableRow "/Game/Blueprints/Systems/Inventory/DT_ItemResource.DT_ItemResource" _array_element)
            (:then
              (if (Utilities|Enum|Equal(Enum) (.id _returnvalue_2) (Utilities|Enum|ByteToEnumE_Items (Math|Conversions|ToByte(Integer) (.itemid _returnvalue))))
                (bind _result (Math|Integer|IncrementInt (Variables|Default|GetCurrentTradeItemIndex))
                  (:%20%20
                    (if (>= _result (Utilities|Array|Length _outrownames))
                      (Variables|Default|SetCurrentTradeItemIndex 1))
                    (CallFunction|EventTradeItem (.itemid _returnvalue) (.tradetooltip _returnvalue))
                    (return)))))))))))

(fn ResetTradedFishCount
  (Variables|Default|SetTradedFish 0))

(fn GetDisplayText
  (return "Trade"))