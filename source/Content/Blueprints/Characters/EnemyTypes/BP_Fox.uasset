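; BP_Fox is a fox character that alternates between walking, running and periodic resting.
; Self-rescheduling random timers toggle the max walk speed between walk and run.
; A delay-driven cycle clears those timers, pauses the AIC_DailyRoutine brain logic while resting, then restarts it after a get-up delay and resumes running.
; Tick and OnInteract are empty, and a ground-trace mesh alignment snippet is left unconnected.
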(event Custom|Event%20StartRunning
  ;[1 0.6238 0.205] Handle Movement Speed Changes
  (Variables|/Script/Engine.CharacterMovementComponent|SetMaxWalkSpeed (Variables|Character|GetCharacterMovement) 5e+02)
  (bind _returnvalue (Utilities|Time|SetTimerbyEvent (delegate Custom|Event%20StopRunning) (Math|Random|RandomFloatinRange 1e+01 3e+01))))

(event Custom|Event%20StopRunning
  ;[1 0.6238 0.205] Handle Movement Speed Changes
  (Variables|/Script/Engine.CharacterMovementComponent|SetMaxWalkSpeed (Variables|Character|GetCharacterMovement) 125.0)
  (bind _returnvalue (Utilities|Time|SetTimerbyEvent (delegate Custom|Event%20StartRunning) (Math|Random|RandomFloatinRange 1e+01 3e+01))))

(event Custom|Event%20StartResting
  ;[0.108 0.3662 1] Resting
  (Utilities|Time|ClearandInvalidateTimerbyHandle (stale Custom|Event%20StartRunning _returnvalue))
  (Utilities|Time|ClearandInvalidateTimerbyHandle (stale Custom|Event%20StopRunning _returnvalue))
  (bind _asaic_daily_routine (Utilities|Casting|CastToAIC_DailyRoutine (Pawn|GetController)))
  (AI|Logic|StopLogic (Variables|/Script/AIModule.AIController|GetBrainComponent _asaic_daily_routine) "Fox resting")
  (Variables|Default|SetIsResting true)
  (Utilities|FlowControl|Delay (Variables|Default|GetTimeToRest))
  (CallFunction|EventStopResting))

(event Custom|Event%20StopResting
  ;[0.108 0.3662 1] Resting
  (Variables|Default|SetIsResting false)
  ;;[1 0.5448 0.1406] Wait for fox to get up
  (Utilities|FlowControl|Delay 1.0)
  (bind _asaic_daily_routine (Utilities|Casting|CastToAIC_DailyRoutine (Pawn|GetController)))
  (Class|BrainComponent|RestartLogic (Variables|/Script/AIModule.AIController|GetBrainComponent _asaic_daily_routine))
  (CallFunction|EventStartRunning)
  (CallFunction|EventStartRestDelay))

(event Custom|Event%20StartRestDelay
  ;[0.108 0.3662 1] Resting
  (Utilities|FlowControl|Delay (Variables|Default|GetTimeBeforeResting))
  (CallFunction|EventStartResting))

(event EventBeginPlay
  (CallFunction|EventStopRunning)
  (CallFunction|EventStartRestDelay))

(event EventTick
  (params (DeltaSeconds :type Float%20%28single-precision%29)))

(event EventOnInteract
  (params (Interactor :type Object%20Object%20Reference)))

(fn ConstructionScript
  (|CallParentFunction))