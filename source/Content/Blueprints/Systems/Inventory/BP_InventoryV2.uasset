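; Slot-based inventory that stores stacked items as DT_ItemResource row handles with counts, using an "EMPTY" row for free slots.
; BeginPlay resizes the array to InventorySize and normalizes each found row by its ID.
; User functions convert the item enum to numeric row names and call system functions that find, stack or remove items by row name.
; NumPad debug keys add a random item and print slot row names.
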(event EventBeginPlay
  (CallFunction|InitializeInventory))

(event Input|KeyboardEvents|DebugKeyNumPadFour
  (params (Key :type Key%20Structure) (ActionValue :type Input%20Action%20Value%20Structure))
  (:Pressed
    (for _array_element (Variables|Default|GetInventory)
      (Development|PrintString (Utilities|String|ToString(Name) (.rowname (.item _array_element)))))))

(event Input|KeyboardEvents|NumPadTwo
  (params (Key :type Key%20Structure))
  (:Pressed
    (CallFunction|AddtoInventory(user) (Utilities|Enum|ByteToEnumE_Items (Math|Conversions|ToByte(Integer) (Math|Random|RandomIntegerinRange 1 9))))))

(fn InitializeInventory
  (bind _inventory (Variables|Default|GetInventory))
  (Utilities|Array|Resize (Variables|Default|GetInventory) (Variables|Default|GetInventorySize))
  (for (_array_element _array_index) (Variables|Default|GetInventory)
    (bind _returnvalue (Utilities|GetDataTableRow "/Game/Blueprints/Systems/Inventory/DT_ItemResource.DT_ItemResource" (.rowname (.Item (Utilities|Struct|BreakS_Inventory _array_element))))
      (:then
        (if (!= (Math|Conversions|ToInteger(Byte) (.ID (Utilities|Struct|BreakS_ItemBase _returnvalue))) 0)
          (Utilities|Array|SetArrayElem _inventory _array_index (Utilities|Struct|MakeS_Inventory (Utilities|Struct|MakeDataTableRowHandle "/Game/Blueprints/Systems/Inventory/DT_ItemResource.DT_ItemResource" (Utilities|String|StringToName (Utilities|String|ToString(Integer) (Math|Conversions|ToInteger(Byte) (.ID (Utilities|Struct|BreakS_ItemBase _returnvalue)))))) (.ItemCount (Utilities|Struct|BreakS_Inventory _array_element))))
          (else
            (Utilities|Array|SetArrayElem _inventory _array_index (Utilities|Struct|MakeS_Inventory (Utilities|Struct|MakeDataTableRowHandle "/Game/Blueprints/Systems/Inventory/DT_ItemResource.DT_ItemResource" "EMPTY") 0))))))))

(fn GetItemName(ID)
  (params (ItemID :type Integer))
  (bind _returnvalue (Utilities|GetDataTableRow "/Game/Blueprints/Systems/Inventory/DT_ItemResource.DT_ItemResource" (Utilities|String|StringToName (Utilities|String|ToString(Integer) ItemID)))
    (:then
      (return (.name _returnvalue)))))

(fn AddtoInventory(system)
  (params (Item :type S%20Inventory%20Structure))
  (bind _inventory (Variables|Default|GetInventory))
  (bind (_localamount1 _index1 _isfound1) (CallFunction|FindItem(system) Item))
  (if _isfound1
    (bind _result (Math|Integer|IncrementInt (.itemcount (Utilities|Array|Get(acopy) _inventory _index1)))
      (:%20%20
        (Utilities|Array|SetArrayElem _inventory _index1 (Utilities|Struct|MakeS_Inventory (.item (Utilities|Array|Get(acopy) _inventory _index1)) _result))
        (return true)))
    (else
      (bind (_isfound1_2 _localindex1) (CallFunction|FindEmptySlot))
      (if _isfound1_2
        (Utilities|Array|SetArrayElem (Variables|Default|GetInventory) _localindex1 (Utilities|Struct|MakeS_Inventory (.Item (Utilities|Struct|BreakS_Inventory Item)) 1))
        (return true)
        (else
          (return false))))))

(fn RemovefromInventory(system)
  (params (Item :type S%20Inventory%20Structure) (Count :type Integer))
  (bind _inventory (Variables|Default|GetInventory))
  (bind (_localamount1 _index1 _isfound1) (CallFunction|FindItem(system) Item))
  (if _isfound1
    (if (>= (|(ItemCount-RemoveCount) (.itemcount (Utilities|Array|Get(acopy) _inventory _index1)) Count) 0)
      (if (== (|(ItemCount-RemoveCount) (.itemcount (Utilities|Array|Get(acopy) _inventory _index1)) Count) 0)
        (Utilities|Array|SetArrayElem _inventory _index1 (Utilities|Struct|MakeS_Inventory (Utilities|Struct|MakeDataTableRowHandle "/Game/Blueprints/Systems/Inventory/DT_ItemResource.DT_ItemResource" "EMPTY") 0))
        (return true)
        (else
          (Utilities|Array|SetArrayElem _inventory _index1 (Utilities|Struct|MakeS_Inventory (.item (Utilities|Array|Get(acopy) _inventory _index1)) (|(ItemCount-RemoveCount) (.itemcount (Utilities|Array|Get(acopy) _inventory _index1)) Count)))
          (return true)))
      (else
        (Development|PrintString "REMOVE_ITEM: TRYING REMOVE MORE THAN YOU CURRENTLY HAVE" true true "(R=1.000000,G=0.000000,B=0.082504,A=1.000000)" 5.0)
        (return false)))
    (else
      (Development|PrintString "REMOVE_ITEM: ITEM NOT FOUND" true true "(R=1.000000,G=0.000000,B=0.058691,A=1.000000)" 5.0)
      (return false))))

(fn GetItemCount(ID)
  (params (Item :type S%20Inventory%20Structure))
  (bind (_localamount1 _index1 _isfound1) (CallFunction|FindItem(system) Item))
  (if _isfound1
    (return _localamount1)
    (else
      (Development|PrintString "GET_ITEM_COUNT: ITEM NOT FOUND IN INVENTORY: RETURN -1" true true "(R=1.000000,G=0.000000,B=0.058691,A=1.000000)" 5.0)
      (return -1))))

(fn FindItem(system)
  (params (Row%20Handle :type S%20Inventory%20Structure))
  (bind (_array_element _array_index) (Utilities|Array|ForEachLoopwithBreak (Variables|Default|GetInventory) :!label _label)
    (:LoopBody
      (if (== (.rowname (.item _array_element)) (.rowname (.item Row%20Handle)))
        (LocalVariables|SetIsFound true)
        (LocalVariables|SetIndex _array_index)
        (LocalVariables|SetLocalAmount (.itemcount _array_element))
        (goto _label Break)))
    (:Completed
      (return (LocalVariables|GetLocalAmount) (LocalVariables|GetIndex) (LocalVariables|GetIsFound)))))

(fn FindEmptySlot
  (bind (_array_element _array_index) (Utilities|Array|ForEachLoopwithBreak (Variables|Default|GetInventory) :!label _label)
    (:LoopBody
      (if (== (.rowname (.item _array_element)) "EMPTY")
        (LocalVariables|SetisFound true)
        (LocalVariables|SetlocalIndex _array_index)
        (goto _label Break)))
    (:Completed
      (return (LocalVariables|GetisFound) (LocalVariables|GetlocalIndex)))))

(fn AddtoInventory(user)
  (params (Item :type E_Items%20Enum :default "NewEnumerator0"))
  (bind _succes (CallFunction|AddtoInventory(system) (Utilities|Struct|MakeS_Inventory (Utilities|Struct|MakeDataTableRowHandle "/Game/Blueprints/Systems/Inventory/DT_ItemResource.DT_ItemResource" (Utilities|String|StringToName (Utilities|String|ToString(Integer) (Math|Conversions|ToInteger(Byte) Item)))) 1)))
  (if _succes
    (Development|PrintString (Utilities|String|Append "Added to inventory: " (Utilities|String|EnumtoString Item)))))

(fn FindItem(user)
  (params (Item :type E_Items%20Enum :default "NewEnumerator0"))
  (bind (_localamount1 _index1 _isfound1) (CallFunction|FindItem(system) (Utilities|Struct|MakeS_Inventory (Utilities|Struct|MakeDataTableRowHandle "/Game/Blueprints/Systems/Inventory/DT_ItemResource.DT_ItemResource" (Utilities|String|StringToName (Utilities|String|ToString(Integer) (Math|Conversions|ToInteger(Byte) Item)))) 0)))
  (return _localamount1 _index1 _isfound1))

(fn RemovefromInventory(user)
  (params (Item :type E_Items%20Enum :default "NewEnumerator0") (Count :type Integer))
  (bind _success_ (CallFunction|RemovefromInventory(system) (Utilities|Struct|MakeS_Inventory (Utilities|Struct|MakeDataTableRowHandle "/Game/Blueprints/Systems/Inventory/DT_ItemResource.DT_ItemResource" (Utilities|String|StringToName (Utilities|String|ToString(Integer) (Math|Conversions|ToInteger(Byte) Item)))) 0) Count))
  (if _success_
    (Development|PrintString (Utilities|String|Append "REMOVE_FROM_INVENTORY(USER): ITEM " (Utilities|String|EnumtoString Item) " SUCCESSFULLY DELETED!"))
    (return true)
    (else
      (Development|PrintString "REMOVE_FROM_INVENTORY(USER): ERROR????" true true "(R=1.000000,G=0.000000,B=0.022203,A=1.000000)" 5.0)
      (return false))))