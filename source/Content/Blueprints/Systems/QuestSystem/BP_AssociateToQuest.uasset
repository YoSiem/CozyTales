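; Component that ties its owning actor to one or more quests, enabling or disabling the actor based on their status.
; It registers with the quest manager through I_QuestAssociated on BeginPlay, after a one-tick delay, and unregisters on EndPlay.
; Quest activation and deactivation events re-run ShouldBeEnabled, which weighs each quest's status against spawn, hide and persist flags.
; An AND flag selects whether all listed quests or any one must qualify.
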(event EventEndPlay
  (params (EndPlayReason :type EEndPlayReason%20Enum :default "Destroyed"))
  (bind _asi_quest_associated (Utilities|Casting|CastToI_QuestAssociated self))
  (Default|UnregisterQuestElement (CallFunction|GetQuestManager) _asi_quest_associated))

(event EventQuestActivated
  (bind _available (CallFunction|ShouldbeEnabled))
  (CallFunction|SetEnabled _available (Components|GetOwner)))

(event EventBeginPlay
  (bind _quest_manager (CallFunction|GetQuestManager))
  (Utilities|FlowControl|DelayUntilNextTick)
  (bind _available (CallFunction|ShouldbeEnabled))
  (CallFunction|SetEnabled _available (Components|GetOwner))
  (bind _asi_quest_associated (Utilities|Casting|CastToI_QuestAssociated self))
  (Utilities|IsValid _quest_manager
    (:Is%20Valid
      (Default|RegisterQuestElement _quest_manager _asi_quest_associated))))

(event EventQuestDeactivated
  (bind _available (CallFunction|ShouldbeEnabled))
  (CallFunction|SetEnabled _available (Components|GetOwner)))

(fn ShouldbeEnabled
  (bind _quest_manager (CallFunction|GetQuestManager))
  (bind _and (Variables|Default|GetAND))
  (bind _array_element (Utilities|Array|ForEachLoopwithBreak (Variables|Default|GetQuestID) :!label _label)
    (:LoopBody
      (Utilities|IsValid _quest_manager
        (:Is%20Valid
          (bind _quest (Default|GetQuestfromArray(ID) _quest_manager _array_element))
          (if (Math|Boolean|ORBoolean (Math|Boolean|ANDBoolean (Utilities|Enum|Equal(Enum) (.QuestStatus (Utilities|Struct|BreakS_Quest _quest)) "NewEnumerator1") (not (Variables|Default|GetSpawnOnlyOnceQuestIsCompleted?)) (not (Variables|Default|GetHideForQuest))) (Math|Boolean|ANDBoolean (Utilities|Enum|Equal(Enum) (.QuestStatus (Utilities|Struct|BreakS_Quest _quest)) "NewEnumerator0") (Variables|Default|GetSpawnFromStart) (not (Utilities|Enum|Equal(Enum) (.QuestStatus (Utilities|Struct|BreakS_Quest _quest)) "NewEnumerator4"))) (and (Utilities|Enum|Equal(Enum) (.QuestStatus (Utilities|Struct|BreakS_Quest _quest)) "NewEnumerator4") (and (or (Variables|Default|GetSpawnOnlyOnceQuestIsCompleted?) (Variables|Default|GetShouldPersistAfterQuestIsDone?)) (not (Variables|Default|GetHideForQuest)))))
            (LocalVariables|SetQuest%20Available true)
            (if (not _and)
              (goto _label Break))
            (else
              (LocalVariables|SetQuest%20Not%20Available true)
              (if _and
                (goto _label Break)))))))
    (:Completed
      (return (and (LocalVariables|GetQuest%20Available) (not (LocalVariables|GetQuest%20Not%20Available)))))))

(fn CheckifAllAssociatedQuestsAreDone
  (for _array_element (Variables|Default|GetQuestID)
    (bind _quest (Default|GetQuestfromArray(ID) (CallFunction|GetQuestManager) _array_element))
    (if (Utilities|Enum|NotEqual(Enum) (.QuestStatus (Utilities|Struct|BreakS_Quest _quest)) "NewEnumerator4")
      (return false)))
  (return true))

(fn GetAssociatedQuests
  (return (Variables|Default|GetQuestID)))