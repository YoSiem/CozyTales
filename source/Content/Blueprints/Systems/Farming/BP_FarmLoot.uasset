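; BP_FarmLoot is a farming pickup that gives the player one plant of its configured PlantType.
; On BeginPlay it applies its LootMesh to the Sphere mesh component.
; When a BP_PlayerCharacter overlaps its Box, it adds the plant through AddPlantOfType, prints an on-screen pickup message and destroys itself.
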(event OnComponentBeginOverlap(Box)
  (params (OverlappedComponent :type Primitive%20Component%20Object%20Reference) (OtherActor :type Actor%20Object%20Reference) (OtherComp :type Primitive%20Component%20Object%20Reference) (OtherBodyIndex :type Integer) (bFromSweep :type Boolean) (SweepResult :type Hit%20Result%20Structure%20%28by%20ref%29))
  (bind _planttype (Variables|Default|GetPlantType))
  (bind _asbp_player_character (Utilities|Casting|CastToBP_PlayerCharacter OtherActor))
  (Default|AddPlantOfType _asbp_player_character _planttype 1)
  (Development|PrintString (Utilities|String|Append "You got: " (Utilities|String|EnumtoString _planttype) " to your inventory:" "+1") true true "(R=0.033181,G=0.000000,B=1.000000,A=1.000000)" 8.0)
  (Actor|DestroyActor))

(event EventBeginPlay
  (Components|StaticMesh|SetStaticMesh (Variables|Default|GetSphere) (Variables|Default|GetLootMesh)))

(fn ConstructionScript)