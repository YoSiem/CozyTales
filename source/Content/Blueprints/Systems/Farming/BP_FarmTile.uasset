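; BP_FarmTile is a farm plot where planting grows a randomly chosen plant that can be harvested once mature.
; Plant type and growth level form DT_PlantsInfo row names supplying meshes and grow times.
; PlantSeedLogic swaps spawned mesh components through three stages, each timed by a one-second Delay countdown.
; Activate harvests ripe plants into BP_FarmLoot and re-enables the interaction overlaps that planting disables.
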(event Custom|Plant
  (bind _output_get (Variables|Default|SetPlantType (Utilities|Enum|ByteToEnumE_PlantTypes (Math|Conversions|ToByte(Integer) (Math|Random|RandomIntegerinRange 1 (- (|GetNumEnumEntries) 1))))))
  (bind _returnvalue (Class|DataTableFunctionLibrary|DoesDataTableRowExist "/Game/Blueprints/Systems/Farming/DT_PlantsInfo.DT_PlantsInfo" (CallFunction|GetDataRowName _output_get "NewEnumerator1")))
  (if _returnvalue
    (|PlantSeedLogic)
    (else
      (Development|PrintString "DEBUG ERROR: This Plant Dont Exist in DataTable"))))

(event EventPlantSeed
  (if (not (Variables|Default|GetIsSomethingPlanted?))
    (Variables|Default|SetIsSomethingPlanted? true)
    (CallFunction|Plant)
    (Variables|/Script/Engine.PrimitiveComponent|SetbGenerateOverlapEvents (Variables|Default|GetInteractionZone) false)))

(event EventActivate
  (CallFunction|Harvest)
  (Variables|/Script/Engine.PrimitiveComponent|SetbGenerateOverlapEvents (Variables|Default|GetInteractionZone) true))

(fn ConstructionScript)

(fn GetPlayerSeedTypeasInt
  (bind _asbp_player_character (Utilities|Casting|CastToBP_PlayerCharacter (Game|GetPlayerCharacter 0)))
  (return (Math|Conversions|ToInteger(Byte) (Variables|/Game/Blueprints/Characters/HeroCharacter/BP_PlayerCharacter.BP_PlayerCharacter_C|GetSeed _asbp_player_character))))

(fn GetPlayerSeedTypeasEnum
  (bind _asbp_player_character (Utilities|Casting|CastToBP_PlayerCharacter (Game|GetPlayerCharacter 0)))
  (return (Variables|/Game/Blueprints/Characters/HeroCharacter/BP_PlayerCharacter.BP_PlayerCharacter_C|GetSeed _asbp_player_character)))

(fn GetDataRowName
  (params (PlantType :type E_PlantTypes%20Enum :default "NewEnumerator3") (GrowthLevel :type E_PlantGrowth%20Enum :default "NewEnumerator0"))
  (return (Utilities|String|StringToName (Utilities|String|Append "Plant" (Utilities|String|ToString(Integer) (Math|Conversions|ToInteger(Byte) PlantType)) "_lv" (Utilities|String|ToString(Integer) (Math|Conversions|ToInteger(Byte) GrowthLevel))))))

(fn GetDataRow
  (params (PlantType :type E_PlantTypes%20Enum :default "NewEnumerator3") (PlantGrowth :type E_PlantGrowth%20Enum :default "NewEnumerator0"))
  (bind _returnvalue (Utilities|GetDataTableRow "/Game/Blueprints/Systems/Farming/DT_PlantsInfo.DT_PlantsInfo" (CallFunction|GetDataRowName PlantType PlantGrowth))
    (:then
      (return _returnvalue))))

(fn UpdateMeshBasedonGrowth
  (params (GrowthLevel :type E_PlantGrowth%20Enum :default "NewEnumerator0"))
  (bind _returnvalue (AddComponent|AddStaticMeshComponent false (Math|Transform|MakeTransform (Variables|Default|GetRelativeTransformLocation) "0, 0, 0" "1.000000,1.000000,1.000000")))
  (bind _output_get (Variables|Default|SetPlantMeshRef _returnvalue))
  (bind _datarow (CallFunction|GetDataRow (Variables|Default|GetPlantType) GrowthLevel))
  (Components|StaticMesh|SetStaticMesh _returnvalue (.plantmesh _datarow))
  (return _output_get (.growtime _datarow)))

(fn Harvest
  (if (Variables|Default|GetReady%20To%20Harvest?)
    (Components|DestroyComponent (Variables|Default|GetPlantMeshRef))
    (bind _datarow (CallFunction|GetDataRow (Variables|Default|GetPlantType) "NewEnumerator3"))
    (Game|SpawnActorfromClass "/Game/Blueprints/Systems/Farming/BP_FarmLoot.BP_FarmLoot_C" (Math|Transform|MakeTransform (Transformation|GetActorLocation) "0, 0, 0" "1.000000,1.000000,1.000000") "Undefined" "MultiplyWithRoot" 0 (Variables|Default|GetPlantType) (.lootmesh _datarow) 0)
    (Variables|Default|SetReady%20To%20Harvest? false)
    (Variables|Default|SetPlantMeshRef 0)
    (Variables|Default|SetIsSomethingPlanted? false)
    (Variables|Default|SetPlantType "NewEnumerator3")))

(fn GetDisplayText
  (if (not (Variables|Default|GetIsSomethingPlanted?))
    (return "Plant Seed")))